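; BP_NPC2 is a platformer NPC that shows an interaction prompt and plays timed dialogue to the player.
; NPCTriggerZone's begin overlap shows the prompt for the cached player, while hiding is bound to InteractionPrompt's own end overlap.
; ResetDialogue restarts the lines, and UpdateDialogue writes each into the player's CurrentDialogueText, re-calling itself after a delay until it clears the text.
; Nothing in this graph calls ResetDialogue.
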(event `self.ReceiveBeginPlay`
  ; Player Reference
  (bind _asbp_third_person_character (cast `/Game/Platformer/Blueprints/BP_ThirdPersonCharacter` (`GameplayStatics.GetPlayerPawn` 0)))
  (set `self.PlayerReference` _asbp_third_person_character))

(event `self.NPCTriggerZone.OnComponentBeginOverlap`
  (params (OverlappedComponent :type "PrimitiveComponent Object Reference") (OtherActor :type "Actor Object Reference") (OtherComp :type "PrimitiveComponent Object Reference") (OtherBodyIndex :type Integer) (bFromSweep :type Boolean) (SweepResult :type "HitResult Structure (by ref)"))
  ; TriggerZone
  (if (== OtherActor (`self.PlayerReference`))
    (`SceneComponent.SetVisibility` (`self.InteractionPrompt`) true false)))

(event `self.InteractionPrompt.OnComponentEndOverlap`
  (params (OverlappedComponent :type "PrimitiveComponent Object Reference") (OtherActor :type "Actor Object Reference") (OtherComp :type "PrimitiveComponent Object Reference") (OtherBodyIndex :type Integer))
  ; TriggerZone
  (if (== OtherActor (`self.PlayerReference`))
    (`SceneComponent.SetVisibility` (`self.InteractionPrompt`) false false)))

(event `UpdateDialogue`
  ; Update Dialogue
  (set `/Game/Platformer/Blueprints/BP_ThirdPersonCharacter.CurrentDialogueText` (`|GetArrayItem` (`self.DialogueLines`) (`self.CurrentDialogueLine`)) (`self.PlayerReference`))
  (set `self.CurrentDialogueLine` (+ (`self.CurrentDialogueLine`) 1))
  (`KismetSystemLibrary.Delay` 2.0)
  (if (!= (`self.CurrentDialogueLine`) (`KismetArrayLibrary.Array_Length` (`self.DialogueLines`)))
    (`self.UpdateDialogue`)
    (else
      (set `/Game/Platformer/Blueprints/BP_ThirdPersonCharacter.CurrentDialogueText` "" (`self.PlayerReference`)))))

(event `ResetDialogue`
  ; Reset Dialogue
  (set `self.CurrentDialogueLine` 0)
  (`self.UpdateDialogue`))

(fn `UserConstructionScript`)