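; Checkpoint actor that records its transform as the third-person character's current checkpoint when that character overlaps its box.
; A timeline started on BeginPlay drives the point light's intensity as a flicker.
; On activation the timeline stops and the light switches to a steady orange at a fixed intensity, marking the checkpoint as reached.
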(event `self.ReceiveBeginPlay`
  (bind (_direction _intensity) (`Timeline|LightFlicker` :!label _label)
    (:`Update`
      (`LightComponent.SetIntensity` (`self.PointLight`) _intensity))))

(event `self.Box.OnComponentBeginOverlap`
  (params (OverlappedComponent :type "PrimitiveComponent Object Reference") (OtherActor :type "Actor Object Reference") (OtherComp :type "PrimitiveComponent Object Reference") (OtherBodyIndex :type Integer) (bFromSweep :type Boolean) (SweepResult :type "HitResult Structure (by ref)"))
  ; Setting CurrentCheckpoint
  (bind _asbp_third_person_character (cast `/Game/Platformer/Blueprints/BP_ThirdPersonCharacter` OtherActor))
  (set `/Game/Platformer/Blueprints/BP_ThirdPersonCharacter.CurrentCheckpoint` (`self.GetTransform`) _asbp_third_person_character)
  ; Checkpoint Light
  (`LightComponent.SetLightColor` (`self.PointLight`) (struct :`R` 0.802083 :`G` 0.371051 :`B` 0.003691 :`A` 1.0) true)
  (`LightComponent.SetIntensity` (`self.PointLight`) 4000.0)
  (goto _label :!via `Stop`))

(fn `UserConstructionScript`)